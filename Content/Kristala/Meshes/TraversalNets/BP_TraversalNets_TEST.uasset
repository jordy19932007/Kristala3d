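; Test Blueprint for a modular traversal net in Kristala, assembled procedurally from mesh tiles.
; The construction script uses HorizontalCount and VerticalCount to lay out a grid of fixed-spacing tiles along local X and downward on Z.
; Separate instanced mesh components supply the corner, edge and center pieces, with inner pieces filled in by loops.
; It has no runtime logic, as all event nodes are disabled.
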(fn `UserConstructionScript`
  (bind _horizontalcount (`self.HorizontalCount`))
  (bind _verticalcount (`self.VerticalCount`))
  (bind _returnvalue (`KismetMathLibrary.Conv_IntToDouble` (* (- (`self.VerticalCount`) 1) -50)))
  (`|ExecutionSequence`
    (:`then_0`
      (`InstancedStaticMeshComponent.AddInstance` (`self.TopLeft`) (`KismetMathLibrary.MakeTransform` (0.0 0.0 0.0)) false)
      (`InstancedStaticMeshComponent.AddInstance` (`self.TopRight`) (`KismetMathLibrary.MakeTransform` (`KismetMathLibrary.MakeVector` (`KismetMathLibrary.Conv_IntToDouble` (* (- _horizontalcount 1) 50)))) false)
      (if (> _horizontalcount 2)
        (for _index (range 1 (+ (- _horizontalcount 2) 1))
          (`InstancedStaticMeshComponent.AddInstance` (`self.TopCenter`) (`KismetMathLibrary.MakeTransform` (`KismetMathLibrary.MakeVector` (`KismetMathLibrary.Conv_IntToDouble` (* _index 50)))) false))))
    (:`then_1`
      (if (> _verticalcount 2)
        (for _index_2 (range 1 (+ (- _verticalcount 2) 1))
          (bind _returnvalue_2 (* _index_2 -50))
          (`InstancedStaticMeshComponent.AddInstance` (`self.CenterLeft`) (`KismetMathLibrary.MakeTransform` (`KismetMathLibrary.MakeVector` 0.0 0.0 (`KismetMathLibrary.Conv_IntToDouble` _returnvalue_2))) false)
          (bind _returnvalue_3 (`KismetMathLibrary.Conv_IntToDouble` _returnvalue_2))
          (`InstancedStaticMeshComponent.AddInstance` (`self.CenterRight`) (`KismetMathLibrary.MakeTransform` (`KismetMathLibrary.MakeVector` (`KismetMathLibrary.Conv_IntToDouble` (* (- (`self.HorizontalCount`) 1) 50)) 0.0 _returnvalue_3)) false)
          (for _index_3 (range 1 (+ (- (`self.HorizontalCount`) 2) 1))
            (`InstancedStaticMeshComponent.AddInstance` (`self.Center`) (`KismetMathLibrary.MakeTransform` (`KismetMathLibrary.MakeVector` (`KismetMathLibrary.Conv_IntToDouble` (* _index_3 50)) 0.0 _returnvalue_3)) false)))))
    (:`then_2`
      (`InstancedStaticMeshComponent.AddInstance` (`self.BottomLeft`) (`KismetMathLibrary.MakeTransform` (`KismetMathLibrary.MakeVector` 0.0 0.0 _returnvalue)) false)
      (`InstancedStaticMeshComponent.AddInstance` (`self.BottomRight`) (`KismetMathLibrary.MakeTransform` (`KismetMathLibrary.MakeVector` (`KismetMathLibrary.Conv_IntToDouble` (* (- (`self.HorizontalCount`) 1) 50)) 0.0 _returnvalue)) false)
      (for _index_4 (range 1 (+ (- (`self.HorizontalCount`) 2) 1))
        (`InstancedStaticMeshComponent.AddInstance` (`self.BottomCenter`) (`KismetMathLibrary.MakeTransform` (`KismetMathLibrary.MakeVector` (`KismetMathLibrary.Conv_IntToDouble` (* _index_4 50)) 0.0 _returnvalue)) false)))))