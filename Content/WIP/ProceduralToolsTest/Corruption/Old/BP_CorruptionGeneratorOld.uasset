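; Older WIP procedural corruption generator that grows tendrils along an authored spline when the construction script runs.
; Each tendril steps along the spline with seeded random up and sideways jitter and becomes its own spline component.
; The offset-based cone random walk is disconnected, so all tendrils share one start point.
; CreateMeshes can dress tendrils with spline meshes and scatter fungus meshes near the start, but nothing here calls it.
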(fn `BuildCorruption`
  (if (> (`SplineComponent.GetNumberOfSplinePoints` (`self.Spline`)) 1)
    (`self.InitializeData`)
    (`self.CreateTendrils`)))

(fn `ClearMeshes`
  (bind _corruptioncomponetlist (`self.CorruptionComponetList`))
  (bind _funguscomponetlist (`self.FungusComponetList`))
  (`|ExecutionSequence`
    (:`then_0`
      (for _array_element _corruptioncomponetlist
        (`/Engine/EditorBlueprintResources/StandardMacros.IsValid` _array_element
          (:`Is Valid`
            (`ActorComponent.K2_DestroyComponent` _array_element))))
      (`KismetArrayLibrary.Array_Clear` _corruptioncomponetlist))
    (:`then_1`
      (for _array_element_2 _funguscomponetlist
        (`/Engine/EditorBlueprintResources/StandardMacros.IsValid` _array_element_2
          (:`Is Valid`
            (`ActorComponent.K2_DestroyComponent` _array_element_2))))
      (`KismetArrayLibrary.Array_Clear` _funguscomponetlist))))

(fn `CreateFungusMesh`
  (locals (L_FungusCount :type Integer) (L_NewLocation :type "Vector Structure"))
  (bind _spline (`self.Spline`))
  (set `local.L_FungusCount` (`KismetMathLibrary.RandomIntegerInRange` (`self.FungusMinCount`) (`self.FungusMaxCount`)))
  (for _ (range (`local.L_FungusCount`))
    (set `local.L_NewLocation` (+ (`SplineComponent.GetLocationAtSplinePoint` _spline 0 "World") (* (`SplineComponent.GetDirectionAtSplinePoint` _spline 0 "World") (`self.FungusStartOffset`)) (* (`KismetMathLibrary.MakeVector` (.x (`KismetMathLibrary.RandomUnitVectorFromStream` (`self.Stream`))) (.y (`KismetMathLibrary.RandomUnitVectorFromStream` (`self.Stream`))) (`KismetMathLibrary.Abs` (.z (`KismetMathLibrary.RandomUnitVectorFromStream` (`self.Stream`))))) (* (`self.TendrilCount`) (`self.TendrilOffset`) 1.25))))
    (bind _returnvalue (`AddComponent|NODE_AddStaticMeshComponent-0`))
    (`KismetArrayLibrary.Array_Add` (`self.FungusComponetList`) _returnvalue)
    (`StaticMeshComponent.SetStaticMesh` _returnvalue (`self.Get Ramdom Mesh` (`self.FungusMeshes`)))
    (`SceneComponent.K2_SetWorldTransform` _returnvalue (`KismetMathLibrary.MakeTransform` (`local.L_NewLocation`) (`KismetMathLibrary.RandomRotator` false) (`KismetMathLibrary.Conv_DoubleToVector` (`KismetMathLibrary.RandomFloatInRangeFromStream` (`self.Stream`) (`self.FungusMinScale`) (`self.FungusMaxScale`)))) false false)))

(fn `CreateMeshes`
  (`self.ClearMeshes`)
  (`|ExecutionSequence`
    (:`then_0`
      (if (and (`self.IsValidMeshList` (`self.SimpleTendrilMeshes`)) (`self.IsValidMeshList` (`self.FungusTendrilMeshes`)))
        (for _array_element (`self.SplineComponetList`)
          (`self.CreateTendrilMesh` _array_element))))
    (:`then_1`
      (if (`self.IsValidMeshList` (`self.FungusMeshes`))
        (`self.CreateFungusMesh`)))))

(fn `CreateTendrilData`
  (params (Offset :type "Vector Structure"))
  (bind _tendrildatalist (`self.TendrilDataList`))
  (bind _returnvalue (`KismetArrayLibrary.Array_Add` _tendrildatalist (make `/Game/WIP/ProceduralToolsTest/Corruption/STR_TendrilData` _)))
  (bind _points (break `/Game/WIP/ProceduralToolsTest/Corruption/STR_TendrilData` (`|GetArrayItem` _tendrildatalist _returnvalue)))
  (`KismetArrayLibrary.Array_Add` _points (+ (`SplineComponent.GetLocationAtSplinePoint` (`self.Spline`) 0 "World") (`local.Offset`)))
  (for _ (range (+ (`self.IterationLimit`) 1))
    (bind _output (`|GetArrayItem` _points (`KismetArrayLibrary.Array_LastIndex` _points)))
    (if (`self.HasReachLastPoint` _output)
      (break)
      (else
        (`KismetArrayLibrary.Array_Add` _points (`self.GetNewPoint` _output))))))

(fn `CreateTendrilMesh`
  (params (SplineRef :type "SplineComponent Object Reference"))
  (bind _tendrimeshscale (`self.TendriMeshScale`))
  (bind _splineref (`local.SplineRef`))
  (for _index (range (+ (- (`SplineComponent.GetNumberOfSplinePoints` SplineRef) 2) 1))
    (bind _returnvalue (`AddComponent|NODE_AddSplineMeshComponent-0`))
    (`StaticMeshComponent.SetStaticMesh` _returnvalue (select `bool` (<= (`KismetMathLibrary.RandomFloatFromStream` (`self.Stream`)) (`self.TendrilFungusPercent`)) :`false` (`self.Get Ramdom Mesh` (`self.SimpleTendrilMeshes`)) :`true` (`self.Get Ramdom Mesh` (`self.FungusTendrilMeshes`))))
    (bind (_location _tangent) (`SplineComponent.GetLocationAndTangentAtSplinePoint` _splineref _index "World"))
    (bind (_location_2 _tangent_2) (`SplineComponent.GetLocationAndTangentAtSplinePoint` _splineref (+ _index 1) "World"))
    (`SplineMeshComponent.SetStartAndEnd` _returnvalue _location _tangent _location_2 _tangent_2 true)
    (`KismetArrayLibrary.Array_Add` (`self.CorruptionComponetList`) _returnvalue)
    (`SplineMeshComponent.SetStartScale` _returnvalue (`KismetMathLibrary.Conv_DoubleToVector2D` _tendrimeshscale) true)
    (`SplineMeshComponent.SetEndScale` _returnvalue (`KismetMathLibrary.Conv_DoubleToVector2D` _tendrimeshscale) true)))

(fn `CreateTendrils`
  (locals (L_TendrilOffset :type "Vector Structure") (L_StartOffset :type "Vector Structure"))
  (bind _tendrildatalist (`self.TendrilDataList`))
  (set `local.L_TendrilOffset` (* (`KismetMathLibrary.GetRightVector` (`KismetMathLibrary.MakeRotFromX` (`SplineComponent.GetDirectionAtSplinePoint` (`self.Spline`) 0 "Local"))) (`self.TendrilOffset`)))
  (set `local.L_StartOffset` (* (`local.L_TendrilOffset`) (`self.TendrilCount`) 0.5))
  (for _index (range (`self.TendrilCount`))
    (`self.NewFunction` (0.0 0.0 0.0))
    (`self.CreateTendrilSpline` (`.Points_3_6354723C4AE7AD8D23EB1BB7841E1E83` (break `/Game/WIP/ProceduralToolsTest/Corruption/STR_TendrilData` (`|GetArrayItem` _tendrildatalist (`KismetArrayLibrary.Array_LastIndex` _tendrildatalist)))))))

(fn `CreateTendrilSpline`
  (params (Points :type "Array of Vector Structure"))
  (returns (newSpline :type "SplineComponent Object Reference"))
  (locals (L_NewSpline :type "SplineComponent Object Reference"))
  (bind _returnvalue (`AddComponent|NODE_AddSplineComponent-0`))
  (set `local.L_NewSpline` _returnvalue)
  (`SplineComponent.ClearSplinePoints` (`local.L_NewSpline`) true)
  (for _array_element (`local.Points`)
    (`SplineComponent.AddSplinePoint` (`local.L_NewSpline`) _array_element "World" true))
  (`KismetArrayLibrary.Array_Add` (`self.SplineComponetList`) (`local.L_NewSpline`))
  (return (`local.L_NewSpline`)))

(fn `Get Ramdom Mesh`
  (params (Meshes :type "Array of StaticMesh Object Reference"))
  (returns (OutItem :type "StaticMesh Object Reference"))
  (return (`KismetArrayLibrary.Array_RandomFromStream` Meshes (`self.Stream`))))

(fn `GetNewPoint`
  (params (Location :type "Vector Structure (by ref)"))
  (returns (NewLocation :type "Vector Structure"))
  (bind _tendrilmaxupoffset (`self.TendrilMaxUpOffset`))
  (bind _tendrilmaxdegrees (`self.TendrilMaxDegrees`))
  (bind _spline (`self.Spline`))
  (bind _returnvalue (`SplineComponent.FindRotationClosestToWorldLocation` _spline Location "World"))
  (bind _returnvalue_2 (+ (* (`KismetMathLibrary.ProjectVectorOnToPlane` (`KismetMathLibrary.RandomUnitVectorInEllipticalConeInDegreesFromStream` (`self.Stream`) (`KismetMathLibrary.GetForwardVector` _returnvalue) _tendrilmaxdegrees _tendrilmaxdegrees) (`KismetMathLibrary.GetUpVector` _returnvalue)) (`self.TendrilStepSize`)) (`SplineComponent.FindLocationClosestToWorldLocation` _spline Location "World")))
  (return (+ _returnvalue_2 (* (`KismetMathLibrary.GetUpVector` (`SplineComponent.FindRotationClosestToWorldLocation` (`self.Spline`) _returnvalue_2 "World")) (`KismetMathLibrary.FClamp` (`KismetMathLibrary.RandomFloatInRangeFromStream` (`self.Stream`) (* _tendrilmaxupoffset -1.0) _tendrilmaxupoffset) 0.0 _tendrilmaxupoffset)))))

(fn `HasReachLastPoint`
  (params (Location :type "Vector Structure"))
  (returns (Succeed :type Boolean))
  (bind _spline (`self.Spline`))
  (bind _returnvalue (- (`SplineComponent.GetNumberOfSplinePoints` _spline) 1))
  (if (<= (`KismetMathLibrary.Dot_VectorVector` (`KismetMathLibrary.GetDirectionUnitVector` Location (`SplineComponent.GetLocationAtSplinePoint` _spline _returnvalue "World")) (`SplineComponent.GetDirectionAtSplinePoint` _spline _returnvalue "World")) 0.0)
    (return true)
    (else
      (return false))))

(fn `InitializeData`
  (bind _splinecomponetlist (`self.SplineComponetList`))
  (`KismetMathLibrary.SetRandomStreamSeed` (`self.Stream`) (`self.RandomSeed`))
  (`KismetArrayLibrary.Array_Clear` (`self.TendrilDataList`))
  (for _array_element _splinecomponetlist
    (`/Engine/EditorBlueprintResources/StandardMacros.IsValid` _array_element
      (:`Is Valid`
        (`ActorComponent.K2_DestroyComponent` _array_element))))
  (`KismetArrayLibrary.Array_Clear` _splinecomponetlist))

(fn `IsValidMeshList`
  (params (CurruptionMeshes :type "Array of StaticMesh Object Reference"))
  (returns (Valid :type Boolean))
  (for _array_element CurruptionMeshes
    (return (`KismetSystemLibrary.IsValid` _array_element)))
  (return false))

(fn `NewFunction`
  (params (Offset :type "Vector Structure"))
  (locals (L_CurrentDistance :type "Float (single-precision)" :default 0.0))
  (bind _l_currentdistance (`local.L_CurrentDistance`))
  (bind _tendrildatalist (`self.TendrilDataList`))
  (bind _spline (`self.Spline`))
  (bind _returnvalue (`SplineComponent.GetRotationAtDistanceAlongSpline` _spline _l_currentdistance "World"))
  (bind _returnvalue_2 (`SplineComponent.GetSplineLength` (`self.Spline`)))
  (bind _returnvalue_3 (`KismetArrayLibrary.Array_Add` _tendrildatalist (make `/Game/WIP/ProceduralToolsTest/Corruption/STR_TendrilData` (`|MakeArray` (+ (`SplineComponent.GetLocationAtSplinePoint` (`self.Spline`) 0 "World") (`local.Offset`))))))
  (while (< (`local.L_CurrentDistance`) _returnvalue_2)
    (set `local.L_CurrentDistance` (`KismetMathLibrary.FClamp` (+ (`local.L_CurrentDistance`) (`KismetMathLibrary.RandomFloatInRangeFromStream` (`self.Stream`) (`self.TendrilStepSize`) 100.0)) 0.0 _returnvalue_2))
    (`KismetArrayLibrary.Array_Add` (`.Points_3_6354723C4AE7AD8D23EB1BB7841E1E83` (break `/Game/WIP/ProceduralToolsTest/Corruption/STR_TendrilData` (`|GetArrayItem` _tendrildatalist _returnvalue_3))) (+ (`SplineComponent.GetLocationAtDistanceAlongSpline` _spline _l_currentdistance "World") (+ (* (`KismetMathLibrary.GetUpVector` _returnvalue) (`KismetMathLibrary.RandomFloatInRangeFromStream` (`self.Stream`) 0.0 (`self.TendrilMaxUpOffset`))) (* (`KismetMathLibrary.GetRightVector` _returnvalue) (`KismetMathLibrary.RandomFloatInRangeFromStream` (`self.Stream`) (* 100.0 -1.0) 100.0)))))))

(fn `UserConstructionScript`
  (`self.BuildCorruption`))