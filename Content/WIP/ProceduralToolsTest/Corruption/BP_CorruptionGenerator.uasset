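; Procedural corruption generator that grows branching tendrils along an authored spline, with fungus clusters near its start.
; The construction script rebuilds seeded, randomly offset parent and child tendril splines from generated point data.
; A separate CreateMeshes function, not called in this graph, skins them with simple, fungus and end spline meshes and scatters fungus static meshes.
; Fungus count and rotation use unseeded randomness, so they vary between builds.
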(fn `BuildCorruption`
  (if (> (`SplineComponent.GetNumberOfSplinePoints` (`self.Spline`)) 1)
    (`self.InitializeData`)
    (`self.CreateTendrils`)))

(fn `ClearMeshes`
  (bind _tendrilsplinemeshcomps (`self.TendrilSplineMeshComps`))
  (bind _fungusmeshcomps (`self.FungusMeshComps`))
  (`|ExecutionSequence`
    (:`then_0`
      (for _array_element _tendrilsplinemeshcomps
        (`/Engine/EditorBlueprintResources/StandardMacros.IsValid` _array_element
          (:`Is Valid`
            (`ActorComponent.K2_DestroyComponent` _array_element))))
      (`KismetArrayLibrary.Array_Clear` _tendrilsplinemeshcomps))
    (:`then_1`
      (for _array_element_2 _fungusmeshcomps
        (`/Engine/EditorBlueprintResources/StandardMacros.IsValid` _array_element_2
          (:`Is Valid`
            (`ActorComponent.K2_DestroyComponent` _array_element_2))))
      (`KismetArrayLibrary.Array_Clear` _fungusmeshcomps))))

(fn `ComputeNewLocation`
  (params (Location :type "Vector Structure") (InRot :type "Rotator Structure") (Scale :type "Float (double-precision)" :default 1.0) (ComputeZ :type Boolean :default true))
  (returns (NewLocation :type "Vector Structure"))
  (bind _tendrilmaxwidth (`self.TendrilMaxWidth`))
  (return (+ Location (+ (`KismetMathLibrary.SelectVector` (* (`KismetMathLibrary.GetUpVector` InRot) (* (`KismetMathLibrary.RandomFloatInRangeFromStream` (`self.Stream`) 0.0 (`self.TendrilMaxUpOffset`)) (`local.Scale`))) (0.0 0.0 0.0) (`local.ComputeZ`)) (* (`KismetMathLibrary.GetRightVector` InRot) (* (`KismetMathLibrary.RandomFloatInRangeFromStream` (`self.Stream`) (* _tendrilmaxwidth -1.0) _tendrilmaxwidth) (`local.Scale`)))))))

(fn `CreateFungusMesh`
  (locals (L_FungusCount :type Integer) (L_NewLocation :type "Vector Structure"))
  (bind _spline (`self.Spline`))
  (set `local.L_FungusCount` (`KismetMathLibrary.RandomIntegerInRange` (`self.FungusMinCount`) (`self.FungusMaxCount`)))
  (for _ (range (`local.L_FungusCount`))
    (set `local.L_NewLocation` (+ (`SplineComponent.GetLocationAtSplinePoint` _spline 0 "World") (* (`SplineComponent.GetDirectionAtSplinePoint` _spline 0 "World") (`self.FungusStartOffset`)) (* (`KismetMathLibrary.MakeVector` (.x (`KismetMathLibrary.RandomUnitVectorFromStream` (`self.Stream`))) (.y (`KismetMathLibrary.RandomUnitVectorFromStream` (`self.Stream`))) (`KismetMathLibrary.Abs` (.z (`KismetMathLibrary.RandomUnitVectorFromStream` (`self.Stream`))))) (* (`self.TendrilCount`) (`self.TendrilStartOffset`) 1.25))))
    (bind _returnvalue (`AddComponent|NODE_AddStaticMeshComponent-0`))
    (`KismetArrayLibrary.Array_Add` (`self.FungusMeshComps`) _returnvalue)
    (`StaticMeshComponent.SetStaticMesh` _returnvalue (`self.Get Ramdom Mesh` (`self.FungusMeshes`)))
    (`SceneComponent.K2_SetWorldTransform` _returnvalue (`KismetMathLibrary.MakeTransform` (`local.L_NewLocation`) (`KismetMathLibrary.RandomRotator` false) (`KismetMathLibrary.Conv_DoubleToVector` (`KismetMathLibrary.RandomFloatInRangeFromStream` (`self.Stream`) (`self.FungusMinScale`) (`self.FungusMaxScale`)))) false false)))

(fn `CreateMeshes`
  (`self.ClearMeshes`)
  (`|ExecutionSequence`
    (:`then_0`
      (if (and (`self.IsValidMeshList` (`self.SimpleTendrilMeshes`)) (`self.IsValidMeshList` (`self.FungusTendrilMeshes`)))
        (`|ExecutionSequence`
          (:`then_0`
            (for _array_element (`self.TendrilSplineComps`)
              (`self.CreateTendrilMesh` _array_element)))
          (:`then_1`
            (for _array_element_2 (`self.TendrilChildSplineComps`)
              (`self.CreateTendrilMesh` _array_element_2 true))))))
    (:`then_1`
      (if (`self.IsValidMeshList` (`self.FungusMeshes`))
        (`self.CreateFungusMesh`)))))

(fn `CreateTendrilChildData`
  (params (Location :type "Vector Structure") (Direction :type "Vector Structure"))
  (locals (L_RightVector :type "Vector Structure" :default (0.0 0.0 0.0)) (L_LastIndex :type Integer :default 0) (L_Rotation :type "Rotator Structure" :default (struct)))
  (bind _tendrildata (`self.TendrilData`))
  (set `local.L_Rotation` (`KismetMathLibrary.MakeRotFromX` Direction))
  (bind _returnvalue (`KismetArrayLibrary.Array_Add` _tendrildata (make `/Game/WIP/ProceduralToolsTest/Corruption/STR_TendrilData` (`|MakeArray` (`local.Location`)) true)))
  (set `local.L_LastIndex` (`KismetMathLibrary.RandomIntegerInRangeFromStream` (`self.Stream`) 2 6))
  (for _index (range 1 (+ (`local.L_LastIndex`) 1))
    (`KismetArrayLibrary.Array_Add` (`.Points_3_6354723C4AE7AD8D23EB1BB7841E1E83` (break `/Game/WIP/ProceduralToolsTest/Corruption/STR_TendrilData` (`|GetArrayItem` _tendrildata _returnvalue))) (`self.ComputeNewLocation` (+ (`local.Location`) (* (`local.Direction`) (* (`KismetMathLibrary.RandomFloatInRangeFromStream` (`self.Stream`) (`self.TendrilMinStepSize`) (`self.TendrilMaxStepSize`)) (`self.TendrilChildPropScale`)) _index)) (`local.L_Rotation`) (`self.TendrilChildPropScale`) (< _index (* (`local.L_LastIndex`) 0.7))))))

(fn `CreateTendrilData`
  (params (Offset :type "Vector Structure"))
  (locals (L_CurrentDistance :type "Float (single-precision)" :default 0.0) (L_MaxDistance :type "Float (single-precision)" :default 0.0) (L_NewLocation :type "Vector Structure"))
  (bind _l_currentdistance (`local.L_CurrentDistance`))
  (bind _tendrildata (`self.TendrilData`))
  (bind _spline (`self.Spline`))
  (bind _returnvalue (`SplineComponent.GetLocationAtDistanceAlongSpline` _spline _l_currentdistance "World"))
  (bind _returnvalue_2 (`KismetMathLibrary.RandomFloatInRangeFromStream` (`self.Stream`) (`self.TendrilMinStepSize`) (`self.TendrilMaxStepSize`)))
  (bind _returnvalue_3 (`SplineComponent.GetRotationAtDistanceAlongSpline` _spline _l_currentdistance "World"))
  (bind _returnvalue_4 (`KismetArrayLibrary.Array_Add` _tendrildata (make `/Game/WIP/ProceduralToolsTest/Corruption/STR_TendrilData` (`|MakeArray` (+ (`SplineComponent.GetLocationAtSplinePoint` (`self.Spline`) 0 "World") (`local.Offset`))))))
  (set `local.L_MaxDistance` (- (`SplineComponent.GetSplineLength` (`self.Spline`)) _returnvalue_2))
  (while (< (`local.L_CurrentDistance`) (`local.L_MaxDistance`))
    (set `local.L_CurrentDistance` (`KismetMathLibrary.FClamp` (+ (`local.L_CurrentDistance`) _returnvalue_2) 0.0 (`local.L_MaxDistance`)))
    (set `local.L_NewLocation` (`self.ComputeNewLocation` _returnvalue _returnvalue_3))
    (`KismetArrayLibrary.Array_Add` (`.Points_3_6354723C4AE7AD8D23EB1BB7841E1E83` (break `/Game/WIP/ProceduralToolsTest/Corruption/STR_TendrilData` (`|GetArrayItem` _tendrildata _returnvalue_4))) (`local.L_NewLocation`))
    (if (and (<= (`KismetMathLibrary.RandomFloatFromStream` (`self.Stream`)) (`self.TendrilChildPercent`)) (< (`local.L_CurrentDistance`) (`local.L_MaxDistance`)))
      (`self.CreateTendrilChildData` (`local.L_NewLocation`) (* (`KismetMathLibrary.VLerp` (`KismetMathLibrary.GetForwardVector` _returnvalue_3) (`KismetMathLibrary.GetDirectionUnitVector` _returnvalue (`local.L_NewLocation`)) 0.45) (1.0 1.0 0.0))))))

(fn `CreateTendrilMesh`
  (params (SplineRef :type "SplineComponent Object Reference") (Child :type Boolean))
  (locals (L_LastIndex :type Integer))
  (bind _tendrimeshscale (`self.TendriMeshScale`))
  (bind _splineref (`local.SplineRef`))
  (set `local.L_LastIndex` (- (`SplineComponent.GetNumberOfSplinePoints` SplineRef) 2))
  (for _index (range (+ (`local.L_LastIndex`) 1))
    (bind _returnvalue (`AddComponent|NODE_AddSplineMeshComponent-0`))
    (`StaticMeshComponent.SetStaticMesh` _returnvalue (select `bool` (== (`local.L_LastIndex`) _index) :`false` (select `bool` (and (<= (`KismetMathLibrary.RandomFloatFromStream` (`self.Stream`)) (`self.TendrilFungusPercent`)) (not (`local.Child`))) :`false` (`self.Get Ramdom Mesh` (`self.SimpleTendrilMeshes`)) :`true` (`self.Get Ramdom Mesh` (`self.FungusTendrilMeshes`))) :`true` (`self.Get Ramdom Mesh` (`self.EndTendrilMeshes`))))
    (bind (_location _tangent) (`SplineComponent.GetLocationAndTangentAtSplinePoint` _splineref _index "World"))
    (bind (_location_2 _tangent_2) (`SplineComponent.GetLocationAndTangentAtSplinePoint` _splineref (+ _index 1) "World"))
    (`SplineMeshComponent.SetStartAndEnd` _returnvalue _location _tangent _location_2 _tangent_2 true)
    (`KismetArrayLibrary.Array_Add` (`self.TendrilSplineMeshComps`) _returnvalue)
    (`SplineMeshComponent.SetStartScale` _returnvalue (`KismetMathLibrary.Conv_DoubleToVector2D` _tendrimeshscale) true)
    (`SplineMeshComponent.SetEndScale` _returnvalue (`KismetMathLibrary.Conv_DoubleToVector2D` _tendrimeshscale) true)))

(fn `CreateTendrils`
  (locals (L_TendrilOffset :type "Vector Structure") (L_StartOffset :type "Vector Structure"))
  (set `local.L_TendrilOffset` (* (`KismetMathLibrary.GetRightVector` (`KismetMathLibrary.MakeRotFromX` (`SplineComponent.GetDirectionAtSplinePoint` (`self.Spline`) 0 "Local"))) (`self.TendrilStartOffset`)))
  (set `local.L_StartOffset` (* (`local.L_TendrilOffset`) (`self.TendrilCount`) 0.5))
  (`|ExecutionSequence`
    (:`then_0`
      (for _index (range (`self.TendrilCount`))
        (`self.CreateTendrilData` (- (`local.L_StartOffset`) (* (`local.L_StartOffset`) _index)))))
    (:`then_1`
      (for _array_element (`self.TendrilData`)
        (bind (_points _child) (break `/Game/WIP/ProceduralToolsTest/Corruption/STR_TendrilData` _array_element))
        (`self.CreateTendrilSpline` _points _child)))))

(fn `CreateTendrilSpline`
  (params (Points :type "Array of Vector Structure") (Child :type Boolean))
  (locals (L_NewSpline :type "SplineComponent Object Reference"))
  (bind _returnvalue (`AddComponent|NODE_AddSplineComponent-0`))
  (set `local.L_NewSpline` _returnvalue)
  (`SplineComponent.ClearSplinePoints` (`local.L_NewSpline`) true)
  (for _array_element (`local.Points`)
    (`SplineComponent.AddSplinePoint` (`local.L_NewSpline`) _array_element "World" true))
  (`KismetArrayLibrary.Array_Add` (select `bool` (`local.Child`) :`false` (`self.TendrilSplineComps`) :`true` (`self.TendrilChildSplineComps`)) (`local.L_NewSpline`))
  (return))

(fn `Get Ramdom Mesh`
  (params (Meshes :type "Array of StaticMesh Object Reference"))
  (returns (OutItem :type "StaticMesh Object Reference"))
  (return (`KismetArrayLibrary.Array_RandomFromStream` Meshes (`self.Stream`))))

(fn `InitializeData`
  (bind _tendrilchildsplinecomps (`self.TendrilChildSplineComps`))
  (bind _tendrilsplinecomps (`self.TendrilSplineComps`))
  (`KismetMathLibrary.SetRandomStreamSeed` (`self.Stream`) (`self.RandomSeed`))
  (`KismetArrayLibrary.Array_Clear` (`self.TendrilData`))
  (`|ExecutionSequence`
    (:`then_0`
      (for _array_element _tendrilsplinecomps
        (`/Engine/EditorBlueprintResources/StandardMacros.IsValid` _array_element
          (:`Is Valid`
            (`ActorComponent.K2_DestroyComponent` _array_element))))
      (`KismetArrayLibrary.Array_Clear` _tendrilsplinecomps))
    (:`then_1`
      (for _array_element_2 _tendrilchildsplinecomps
        (`/Engine/EditorBlueprintResources/StandardMacros.IsValid` _array_element_2
          (:`Is Valid`
            (`ActorComponent.K2_DestroyComponent` _array_element_2))))
      (`KismetArrayLibrary.Array_Clear` _tendrilchildsplinecomps))))

(fn `IsValidMeshList`
  (params (CurruptionMeshes :type "Array of StaticMesh Object Reference"))
  (returns (Valid :type Boolean))
  (for _array_element CurruptionMeshes
    (return (`KismetSystemLibrary.IsValid` _array_element)))
  (return false))

(fn `UserConstructionScript`
  (`self.BuildCorruption`))