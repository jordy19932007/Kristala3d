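; Environment generator actor that procedurally builds corruption growth, with branching tendrils and fungus clusters, along an editable spline.
; Without a valid merged mesh to display, construction generates seeded, jittered point paths with random child branches and turns them into spline components.
; CreateMeshes, not called by construction, uses a separate seed to dress those splines with start, middle and end spline meshes and scatter fungus at the spline's start.
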(fn `BuildCorruption`
  (if (> (`SplineComponent.GetNumberOfSplinePoints` (`self.Spline`)) 1)
    (`self.InitializeData`)
    (`self.CreateTendrils`)))

(fn `ClearMeshes`
  (bind _tendrilsplinemeshcomps (`self.TendrilSplineMeshComps`))
  (bind _fungusmeshcomps (`self.FungusMeshComps`))
  (`|ExecutionSequence`
    (:`then_0`
      (for _array_element _tendrilsplinemeshcomps
        (`/Engine/EditorBlueprintResources/StandardMacros.IsValid` _array_element
          (:`Is Valid`
            (`ActorComponent.K2_DestroyComponent` _array_element))))
      (`KismetArrayLibrary.Array_Clear` _tendrilsplinemeshcomps))
    (:`then_1`
      (for _array_element_2 _fungusmeshcomps
        (`/Engine/EditorBlueprintResources/StandardMacros.IsValid` _array_element_2
          (:`Is Valid`
            (`ActorComponent.K2_DestroyComponent` _array_element_2))))
      (`KismetArrayLibrary.Array_Clear` _fungusmeshcomps))))

(fn `ComputeNewLocation`
  (params (Location :type "Vector Structure") (InRot :type "Rotator Structure") (Scale :type "Float (double-precision)" :default 1.0) (ComputeZ :type Boolean :default true))
  (returns (NewLocation :type "Vector Structure"))
  (bind _tendrilmaxwidth (`self.TendrilMaxWidth`))
  (return (+ Location (+ (`KismetMathLibrary.SelectVector` (* (`KismetMathLibrary.GetUpVector` InRot) (* (`KismetMathLibrary.RandomFloatInRangeFromStream` (`self.ConstructStream`) 0.0 (`self.TendrilMaxUpOffset`)) (`local.Scale`))) (0.0 0.0 0.0) (`local.ComputeZ`)) (* (`KismetMathLibrary.GetRightVector` InRot) (* (`KismetMathLibrary.RandomFloatInRangeFromStream` (`self.ConstructStream`) (* _tendrilmaxwidth -1.0) _tendrilmaxwidth) (`local.Scale`)))))))

(fn `CreateFungusMesh`
  (locals (L_FungusCount :type Integer) (L_NewLocation :type "Vector Structure") (L_StartOffset :type "Vector Structure") (L_Index :type Integer))
  (set `local.L_FungusCount` (`KismetMathLibrary.RandomIntegerInRangeFromStream` (`self.MeshesStream`) (`self.FungusMinCount`) (`self.FungusMaxCount`)))
  (set `local.L_StartOffset` (`SplineComponent.GetLocationAtSplinePoint` (`self.Spline`) 0 "World"))
  (for _index (range (`local.L_FungusCount`))
    (set `local.L_Index` _index)
    (set `local.L_NewLocation` (+ (`local.L_StartOffset`) (`KismetMathLibrary.SelectVector` (* (`KismetMathLibrary.MakeVector` (.x (`KismetMathLibrary.RandomUnitVectorInConeInDegreesFromStream` (`self.MeshesStream`) (`SplineComponent.GetDirectionAtSplinePoint` (`self.Spline`) 0 "World") 35.0)) (.y (`KismetMathLibrary.RandomUnitVectorInConeInDegreesFromStream` (`self.MeshesStream`) (`SplineComponent.GetDirectionAtSplinePoint` (`self.Spline`) 0 "World") 35.0)) (`KismetMathLibrary.Abs` (.z (`KismetMathLibrary.RandomUnitVectorInConeInDegreesFromStream` (`self.MeshesStream`) (`SplineComponent.GetDirectionAtSplinePoint` (`self.Spline`) 0 "World") 35.0)))) (`self.FungusMaxOffset`)) (0.0 0.0 0.0) (!= (`local.L_Index`) 0))))
    (bind _returnvalue (`AddComponent|NODE_AddStaticMeshComponent-0`))
    (`KismetArrayLibrary.Array_Add` (`self.FungusMeshComps`) _returnvalue)
    (`StaticMeshComponent.SetStaticMesh` _returnvalue (`self.Get Ramdom Mesh` (`self.FungusMeshes`)))
    (`SceneComponent.K2_SetWorldTransform` _returnvalue (`KismetMathLibrary.MakeTransform` (`local.L_NewLocation`) (`KismetMathLibrary.RandomRotatorFromStream` (`self.MeshesStream`)) (`KismetMathLibrary.SelectVector` (`KismetMathLibrary.Conv_DoubleToVector` (`KismetMathLibrary.RandomFloatInRangeFromStream` (`self.MeshesStream`) (`self.FungusMinScale`) (`self.FungusMaxScale`))) (`KismetMathLibrary.Conv_DoubleToVector` (* (`self.TendrilCount`) (`self.TendrilStartOffset`) 0.03)) (!= (`local.L_Index`) 0))) false true)))

(fn `CreateMeshes`
  (locals (L_StartedFungus :type Boolean))
  (bind _returnvalue (not (`local.L_StartedFungus`)))
  (`KismetMathLibrary.SetRandomStreamSeed` (`self.MeshesStream`) (`self.MeshesSeed`))
  (`self.ClearMeshes`)
  (if (and (`self.IsValidMeshList` (`self.SimpleTendrilMeshes`)) (`self.IsValidMeshList` (`self.FungusTendrilMeshes`)) (`self.IsValidMeshList` (`self.StartTendrilMeshes`)) (`self.IsValidMeshList` (`self.EndTendrilMeshes`)) (`self.IsValidMeshList` (`self.FungusMeshes`)))
    (set `local.L_StartedFungus` (> (`KismetMathLibrary.Max` (`self.FungusMinCount`) (`self.FungusMaxCount`)) 0))
    (`|ExecutionSequence`
      (:`then_0`
        ;[1 1 1] Fungus
        (if (`local.L_StartedFungus`)
          (`self.CreateFungusMesh`)))
      (:`then_1`
        ;[1 1 1] Base tendril
        (for _array_element (`self.TendrilSplineComps`)
          (`self.CreateTendrilMesh` _array_element _returnvalue)))
      (:`then_2`
        ;[1 1 1] Child tendril
        (for _array_element_2 (`self.TendrilChildSplineComps`)
          (`self.CreateTendrilMesh` _array_element_2 _returnvalue true))))))

(fn `CreateTendrilChildData`
  (params (Location :type "Vector Structure") (Direction :type "Vector Structure"))
  (locals (L_RightVector :type "Vector Structure" :default (0.0 0.0 0.0)) (L_LastIndex :type Integer :default 0) (L_Rotation :type "Rotator Structure" :default (struct)))
  (bind _tendrildata (`self.TendrilData`))
  (set `local.L_Rotation` (`KismetMathLibrary.MakeRotFromX` Direction))
  (bind _returnvalue (`KismetArrayLibrary.Array_Add` _tendrildata (make `/Game/Kristala/Blueprints/EnvironmentalObject/Corruption/Data/STR_TendrilData` (`|MakeArray` (`local.Location`)) true)))
  (set `local.L_LastIndex` (`KismetMathLibrary.RandomIntegerInRangeFromStream` (`self.ConstructStream`) 2 6))
  (for _index (range 1 (+ (`local.L_LastIndex`) 1))
    (`KismetArrayLibrary.Array_Add` (`.Points_3_6354723C4AE7AD8D23EB1BB7841E1E83` (break `/Game/Kristala/Blueprints/EnvironmentalObject/Corruption/Data/STR_TendrilData` (`|GetArrayItem` _tendrildata _returnvalue))) (`self.ComputeNewLocation` (+ (`local.Location`) (* (`local.Direction`) (* (`KismetMathLibrary.RandomFloatInRangeFromStream` (`self.ConstructStream`) (`self.TendrilMinStepSize`) (`self.TendrilMaxStepSize`)) (`self.TendrilChildPropScale`)) _index)) (`local.L_Rotation`) (`self.TendrilChildPropScale`) (< _index (* (`local.L_LastIndex`) 0.7))))))

(fn `CreateTendrilData`
  (params (Offset :type "Vector Structure"))
  (locals (L_CurrentDistance :type "Float (single-precision)" :default 0.0) (L_MaxDistance :type "Float (single-precision)" :default 0.0) (L_NewLocation :type "Vector Structure"))
  (bind _l_currentdistance (`local.L_CurrentDistance`))
  (bind _tendrildata (`self.TendrilData`))
  (bind _spline (`self.Spline`))
  (bind _returnvalue (`SplineComponent.GetLocationAtDistanceAlongSpline` _spline _l_currentdistance "World"))
  (bind _returnvalue_2 (`KismetMathLibrary.RandomFloatInRangeFromStream` (`self.ConstructStream`) (`self.TendrilMinStepSize`) (`self.TendrilMaxStepSize`)))
  (bind _returnvalue_3 (`SplineComponent.GetRotationAtDistanceAlongSpline` _spline _l_currentdistance "World"))
  (bind _returnvalue_4 (`KismetArrayLibrary.Array_Add` _tendrildata (make `/Game/Kristala/Blueprints/EnvironmentalObject/Corruption/Data/STR_TendrilData` (`|MakeArray` (+ (`SplineComponent.GetLocationAtSplinePoint` (`self.Spline`) 0 "World") (`local.Offset`))))))
  (set `local.L_MaxDistance` (- (`SplineComponent.GetSplineLength` (`self.Spline`)) _returnvalue_2))
  (while (< (`local.L_CurrentDistance`) (`local.L_MaxDistance`))
    (set `local.L_CurrentDistance` (`KismetMathLibrary.FClamp` (+ (`local.L_CurrentDistance`) _returnvalue_2) 0.0 (`local.L_MaxDistance`)))
    (set `local.L_NewLocation` (+ (`local.Offset`) (`self.ComputeNewLocation` _returnvalue _returnvalue_3)))
    (`KismetArrayLibrary.Array_Add` (`.Points_3_6354723C4AE7AD8D23EB1BB7841E1E83` (break `/Game/Kristala/Blueprints/EnvironmentalObject/Corruption/Data/STR_TendrilData` (`|GetArrayItem` _tendrildata _returnvalue_4))) (`local.L_NewLocation`))
    (if (and (<= (`KismetMathLibrary.RandomFloatFromStream` (`self.ConstructStream`)) (`self.TendrilChildPercent`)) (< (`local.L_CurrentDistance`) (`local.L_MaxDistance`)))
      (`self.CreateTendrilChildData` (`local.L_NewLocation`) (* (`KismetMathLibrary.VLerp` (`KismetMathLibrary.GetForwardVector` _returnvalue_3) (`KismetMathLibrary.GetDirectionUnitVector` _returnvalue (`local.L_NewLocation`)) 0.45) (1.0 1.0 0.0))))))

(fn `CreateTendrilMesh`
  (params (SplineRef :type "SplineComponent Object Reference") (FullTendril :type Boolean) (ChildTendril :type Boolean))
  (locals (L_LastIndex :type Integer) (L_Index :type Integer) (L_Splinemesh :type "SplineMeshComponent Object Reference"))
  (bind _l_index (`local.L_Index`))
  (bind _splineref (`local.SplineRef`))
  (bind (_location _tangent) (`SplineComponent.GetLocationAndTangentAtSplinePoint` _splineref _l_index "Local"))
  (bind _returnvalue (`KismetMathLibrary.Conv_DoubleToVector2D` (`self.TendriMeshScale`)))
  (bind (_location_2 _tangent_2) (`SplineComponent.GetLocationAndTangentAtSplinePoint` _splineref (+ _l_index 1) "Local"))
  (set `local.L_LastIndex` (- (`SplineComponent.GetNumberOfSplinePoints` SplineRef) 2))
  (for _index (range (+ (`local.L_LastIndex`) 1))
    (set `local.L_Index` _index)
    (bind _returnvalue_2 (`AddComponent|NODE_AddSplineMeshComponent-0`))
    (set `local.L_Splinemesh` _returnvalue_2)
    (`KismetArrayLibrary.Array_Add` (`self.TendrilSplineMeshComps`) (`local.L_Splinemesh`))
    (`StaticMeshComponent.SetStaticMesh` (`local.L_Splinemesh`) (`self.GetTendrilMesh` (`local.L_Index`) (`local.L_LastIndex`) (`local.FullTendril`) (`local.ChildTendril`)))
    (`SplineMeshComponent.SetStartAndEnd` (`local.L_Splinemesh`) _location _tangent _location_2 _tangent_2 true)
    (`SplineMeshComponent.SetStartScale` (`local.L_Splinemesh`) _returnvalue true)
    (`SplineMeshComponent.SetEndScale` (`local.L_Splinemesh`) _returnvalue true)))

(fn `CreateTendrils`
  (locals (L_TendrilOffset :type "Vector Structure") (L_StartOffset :type "Vector Structure"))
  (set `local.L_TendrilOffset` (* (`KismetMathLibrary.GetRightVector` (`KismetMathLibrary.MakeRotFromX` (`SplineComponent.GetDirectionAtSplinePoint` (`self.Spline`) 0 "Local"))) (`self.TendrilStartOffset`)))
  (set `local.L_StartOffset` (* (`local.L_TendrilOffset`) (`self.TendrilCount`) 0.5))
  (`|ExecutionSequence`
    (:`then_0`
      (for _index (range (`self.TendrilCount`))
        (`self.CreateTendrilData` (- (`local.L_StartOffset`) (* (`local.L_TendrilOffset`) _index)))))
    (:`then_1`
      (for _array_element (`self.TendrilData`)
        (bind (_points _child) (break `/Game/Kristala/Blueprints/EnvironmentalObject/Corruption/Data/STR_TendrilData` _array_element))
        (`self.CreateTendrilSpline` _points _child)))))

(fn `CreateTendrilSpline`
  (params (Points :type "Array of Vector Structure") (Child :type Boolean))
  (locals (L_NewSpline :type "SplineComponent Object Reference"))
  (bind _returnvalue (`AddComponent|NODE_AddSplineComponent-0`))
  (set `local.L_NewSpline` _returnvalue)
  (`SplineComponent.ClearSplinePoints` (`local.L_NewSpline`) true)
  (for _array_element (`local.Points`)
    (`SplineComponent.AddSplinePoint` (`local.L_NewSpline`) _array_element "World" true))
  (`KismetArrayLibrary.Array_Add` (select `bool` (`local.Child`) :`false` (`self.TendrilSplineComps`) :`true` (`self.TendrilChildSplineComps`)) (`local.L_NewSpline`))
  (return))

(fn `Get Ramdom Mesh`
  (params (Meshes :type "Array of StaticMesh Object Reference"))
  (returns (OutItem :type "StaticMesh Object Reference"))
  (return (`KismetArrayLibrary.Array_RandomFromStream` Meshes (`self.MeshesStream`))))

(fn `GetTendrilMesh`
  (params (Index :type Integer) (lastIndex :type Integer) (FullTendril :type Boolean) (ChildTendril :type Boolean))
  (returns (SelectedMesh :type "StaticMesh Object Reference"))
  (locals (L_SelectedMesh :type "StaticMesh Object Reference"))
  (`|ExecutionSequence`
    (:`then_0`
      (if (and (== Index 0) (not ChildTendril))
        (set `local.L_SelectedMesh` (`self.Get Ramdom Mesh` (`self.StartTendrilMeshes`)))
        (elif (== (`local.lastIndex`) (`local.Index`))
          (set `local.L_SelectedMesh` (`self.Get Ramdom Mesh` (`self.EndTendrilMeshes`)))
          (elif (<= (`KismetMathLibrary.RandomFloatFromStream` (`self.MeshesStream`)) (`self.TendrilFungusPercent`))
            (set `local.L_SelectedMesh` (`self.Get Ramdom Mesh` (`self.FungusTendrilMeshes`)))
            (else
              (set `local.L_SelectedMesh` (`self.Get Ramdom Mesh` (`self.SimpleTendrilMeshes`))))))))
    (:`then_1`
      (return (`local.L_SelectedMesh`)))))

(fn `InitializeData`
  (bind _tendrilchildsplinecomps (`self.TendrilChildSplineComps`))
  (bind _tendrilsplinecomps (`self.TendrilSplineComps`))
  (`KismetMathLibrary.SetRandomStreamSeed` (`self.ConstructStream`) (`self.GenerationSeed`))
  (`KismetArrayLibrary.Array_Clear` (`self.TendrilData`))
  (`|ExecutionSequence`
    (:`then_0`
      (for _array_element _tendrilsplinecomps
        (`/Engine/EditorBlueprintResources/StandardMacros.IsValid` _array_element
          (:`Is Valid`
            (`ActorComponent.K2_DestroyComponent` _array_element))))
      (`KismetArrayLibrary.Array_Clear` _tendrilsplinecomps))
    (:`then_1`
      (for _array_element_2 _tendrilchildsplinecomps
        (`/Engine/EditorBlueprintResources/StandardMacros.IsValid` _array_element_2
          (:`Is Valid`
            (`ActorComponent.K2_DestroyComponent` _array_element_2))))
      (`KismetArrayLibrary.Array_Clear` _tendrilchildsplinecomps))))

(fn `IsValidMeshList`
  (params (CurruptionMeshes :type "Array of StaticMesh Object Reference"))
  (returns (Valid :type Boolean))
  (for _array_element CurruptionMeshes
    (return (`KismetSystemLibrary.IsValid` _array_element)))
  (return false))

(fn `UserConstructionScript`
  (`/Engine/EditorBlueprintResources/StandardMacros.IsValid` (`self.MegerMesh`)
    (:`Is Valid`
      (`StaticMeshComponent.SetStaticMesh` (`self.MergeMeshComponent`) (`self.MegerMesh`)))
    (:`Is Not Valid`
      (`self.BuildCorruption`))))